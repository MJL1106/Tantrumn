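; AI controller for Tantrumn that runs the BP_TantrumnBattle behavior tree and feeds its blackboard.
; On BeginPlay it sets the Destination key to the location of the first BP_ThrowableActor found in the level.
; Each tick it mirrors the game state's IsPlaying result into the IsPlaying key.
; An alternative function targets the first level end trigger, but nothing in this Blueprint calls it.
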(event `self.ReceiveBeginPlay`
  (`self.RunBehaviorTree` "/Game/Tantrumn/Blueprints/AI/BP_TantrumnBattle.BP_TantrumnBattle")
  (`self.SetThrowableObjectAsDestination`))

(event `self.ReceiveTick`
  (params (DeltaSeconds :type "Float (single-precision)"))
  (bind _asbp_tantrumn_game_state_base (cast `/Game/Tantrumn/Blueprints/GameModes/BP_TantrumnGameStateBase` (`GameplayStatics.GetGameState`)))
  (`BlackboardComponent.SetValueAsBool` (`self.Blackboard`) "IsPlaying" (`TantrumnGameStateBase.IsPlaying` _asbp_tantrumn_game_state_base)))

(fn `SetRaceEndAsDestination`
  (bind _outactors (`GameplayStatics.GetAllActorsOfClass` "/Script/Tantrumn.TantrumnLevelEndtrigger"))
  (if (> (`KismetArrayLibrary.Array_Length` _outactors) 0)
    (`BlackboardComponent.SetValueAsVector` (`self.Blackboard`) "Destination" (`self.K2_GetActorLocation` (`|GetArrayItem` _outactors)))))

(fn `SetThrowableObjectAsDestination`
  (bind _outactors (`GameplayStatics.GetAllActorsOfClass` "/Game/Tantrumn/Blueprints/GameplayObjects/BP_ThrowableActor.BP_ThrowableActor_C"))
  (if (> (`KismetArrayLibrary.Array_Length` _outactors) 0)
    (`BlackboardComponent.SetValueAsVector` (`self.Blackboard`) "Destination" (`self.K2_GetActorLocation` (`|GetArrayItem` _outactors)))))

(fn `UserConstructionScript`)