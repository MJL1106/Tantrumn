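; Player character Blueprint for Tantrumn, with empty jump and interaction event stubs and interaction functions that return false.
; Its Hold macro separates taps from holds using a retriggerable delay and two gates: releasing early fires Tap, while outlasting the duration fires Held.
; Disconnected debug logic in the event graph prints velocity and times the jump apex, but never runs.
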(event `self.OnJumped`)

(event `self.NonTypedInteract`)

(fn `SignatureInteract`
  (returns (Return :type Boolean))
  (return false))

(fn `TypedInteract`
  (returns (ReturnValue :type Boolean))
  (return false))

(fn `UserConstructionScript`)