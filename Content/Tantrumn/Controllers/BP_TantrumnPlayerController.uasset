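; Player controller Blueprint for Tantrumn whose input logic is entirely disconnected, so it does nothing at runtime.
; The MoveForward, MoveRight and LookUp axis events are empty.
; Orphaned node chains remain for moving the controlled TantrumnCharacterBase along its forward and right vectors, jump start and stop, and pitch and yaw input.
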(event `InputAction|Jump`
  (params (Key :type "Key Structure")))

(event `InputAxis|MoveForward`
  (params (AxisValue :type "Float (single-precision)")))

(event `InputAxis|MoveRight`
  (params (AxisValue :type "Float (single-precision)")))

(event `InputAxis|LookUp`
  (params (AxisValue :type "Float (single-precision)")))

(fn `UserConstructionScript`)